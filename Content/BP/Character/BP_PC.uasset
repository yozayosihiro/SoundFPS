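; BP_PC is the player character for a shooter, handling movement, camera look, sprint, crouch, jump and rifle aim, fire and reload.
; State flags gate actions through CheckMovementCondition, while looping timers drive walk-speed interpolation and automatic fire.
; It spawns a BP_AR4 on BeginPlay and sends movement, aim-offset and IK data to the AnimInstance through interface messages.
; Grenade arc prediction and throw logic exist but are disconnected from their input.
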(fn ConstructionScript)

(fn CalculateMovementValue
  (bind _returnvalue (Transformation|GetVelocity))
  (Variables|FLOAT|SetCurrentPitch (.pitch (Math|Interpolation|RInterpTo (Math|Rotator|MakeRotator 0.0 (Variables|FLOAT|GetCurrentPitch) (Variables|Float|GetCurrentYaw)) (Math|Rotator|Delta(Rotator) (Pawn|GetControlRotation :!class /Script/Engine.Pawn) (Transformation|GetActorRotation)) (Utilities|Time|GetWorldDeltaSeconds) 64.0)))
  (Variables|Float|SetCurrentYaw (.yaw (Math|Interpolation|RInterpTo (Math|Rotator|MakeRotator 0.0 (Variables|FLOAT|GetCurrentPitch) (Variables|Float|GetCurrentYaw)) (Math|Rotator|Delta(Rotator) (Pawn|GetControlRotation :!class /Script/Engine.Pawn) (Transformation|GetActorRotation)) (Utilities|Time|GetWorldDeltaSeconds) 64.0)))
  (return (.yaw (Math|Rotator|Delta(Rotator) (Transformation|GetActorRotation) (Math|Conversions|RotationFromXVector _returnvalue))) (Math|Vector|VectorLengthXY _returnvalue) (Variables|FLOAT|GetCurrentPitch) (Variables|Float|GetCurrentYaw)))

(fn ChangeMovementType
  (params (NewMovementType :type E_MovementType%20Enum :default "NewEnumerator0"))
  ;[0.1302 0.1302 0.1302] Enumの値でSwitchし、Speedを変更
  (bind _output_get (Variables|ENUM|Sete_MovementType NewMovementType))
  (switch Utilities|FlowControl|Switch|SwitchonE_MovementType _output_get
    (:NewEnumerator0
      (Variables|Float|SetCurrentSpeed 5e+02))
    (:NewEnumerator1
      (Variables|Float|SetCurrentSpeed 2.5e+02))
    (:NewEnumerator2
      (Variables|Float|SetCurrentSpeed 1.5e+02))
    (:NewEnumerator3
      (Variables|Float|SetCurrentSpeed 8e+02)))
  ;[0.1146 0.1146 0.1146] Set timer処理、TimeにGet World Delta Secondsを代入することで、Tickと同じ速度で関数を処理させる
  (bind _returnvalue (Utilities|Time|SetTimerbyEvent (EventDispatchers|CreateEvent :!event ChangeMovementSpeed) (Utilities|Time|GetWorldDeltaSeconds) true))
  (Variables|HANDLE|SetH_ChangeMovementSpeed _returnvalue))

(fn ChangeMovementSpeed
  (bind _charactermovement (Variables|Character|GetCharacterMovement))
  (Variables|/Script/Engine.CharacterMovementComponent|SetMaxWalkSpeed _charactermovement (Math|Interpolation|FInterpTo (Variables|/Script/Engine.CharacterMovementComponent|GetMaxWalkSpeed _charactermovement) (Variables|Float|GetCurrentSpeed) (Utilities|Time|GetWorldDeltaSeconds) 16.0)))

(fn PredictGrenadeArc
  (bind _mesh (Variables|Character|GetMesh))
  (bind _returnvalue (Transformation|GetSocketLocation _mesh "GrenadeGrabSocket"))
  (bind _returnvalue_2 (Transformation|GetSocketRotation _mesh "GrenadeGrabSocket"))
  (bind _returnvalue_3 (Math|Vector|GetForwardVector _returnvalue_2))
  (bind _returnvalue_4 (* _returnvalue_3 -2e+01))
  (bind _returnvalue_5 (+ _returnvalue _returnvalue_4))
  (bind _outlaunchvelocity (Game|SuggestProjectileVelocityCustomArc _returnvalue_5 (+ _returnvalue_5 (* (Math|Vector|GetForwardVector (Transformation|GetWorldRotation (Variables|Default|GetCamera))) 1e+03)) 0.0 0.5))
  (bind _output_get (Variables|VECTOR|SetGrenadeLaunchVelocity _outlaunchvelocity))
  (bind (_outhit _outpathpositions _outlasttracedestination) (Class|GameplayStatics|BlueprintPredictProjectilePathbyTraceChannel _returnvalue_5 _output_get true 1e+01 "ECC_WorldDynamic" false (Utilities|Array|MakeArray self) "ForOneFrame" 1e+01))
  (Class|KismetSystemLibrary|DrawDebugCylinder _outlasttracedestination (+ _outlasttracedestination "0, 0,30.000000") 3e+02 30 "(R=0.871560,G=1.000000,B=0.000000,A=1.000000)" (Utilities|Time|GetWorldDeltaSeconds) 1e+01))

(fn ThrowGrenade
  ;[1 1 1] Grenadeクラス内のThrow関数を実行
  (Default|Throw (Variables|REFERENCE|GetGrenade) (Variables|VECTOR|GetGrenadeLaunchVelocity)))

(fn WalkCameraShake
  ;[1 0.2812 0.2812] WSADのいずれかを押している又は、ADS中ではないならば
  (if (and (or (> (Input|AxisValues|GetMoveForward/Backward) 0.0) (> (Input|AxisValues|GetMoveRight/Left) 0.0)) (not (Variables|BOOL|GetAiming)))
    (Class|PlayerCameraManager|PlayCameraShake (Game|GetPlayerCameraManager 0) "/Game/BP/Character/BP_WalkCameraShake.BP_WalkCameraShake_C" 1.0 "CameraLocal" "0, 0, 0")))

(fn UpdateMovementState
  (Variables|STRUCTURE|Sets_MovementState (Utilities|Struct|MakeS_MovementState (Variables|BOOL|GetRunning) (Variables|BOOL|GetCrouching) (Variables|BOOL|GetAiming) (Variables|BOOL|GetFireing) (Variables|BOOL|GetReloading) (Variables|BOOL|GetHoldingGrenade))))

(event Input|ActionEvents|InputActionSprint
  (params (Key :type Key%20Structure))
  (bind _returnvalue (Utilities|GetAnimInstance))
  ;[1 1 1] 走る処理
  (:Pressed
    (Utilities|CheckMovementCondition (Utilities|Struct|MakeS_MovementState false (Variables|BOOL|GetCrouching) (Variables|BOOL|GetAiming) (Variables|BOOL|GetFireing) false false)
      (:DoLogic
        (bind _output_get (Variables|BOOL|SetRunning true))
        ;;[0.03349 0.04049 1] Interface呼び出し
        (Class|BPIAnimation|SetRunning(Message) _returnvalue _output_get)
        (CallFunction|ChangeMovementType "NewEnumerator3")
        (CallFunction|UpdateMovementState :!label _label))))
  (:Released
    (Utilities|CheckMovementCondition (Utilities|Struct|MakeS_MovementState false (Variables|BOOL|GetCrouching) (Variables|BOOL|GetAiming) (Variables|BOOL|GetFireing) false false)
      (:DoLogic
        (bind _output_get_2 (Variables|BOOL|SetRunning false))
        (Class|BPIAnimation|SetRunning(Message) _returnvalue _output_get_2)
        (CallFunction|ChangeMovementType "NewEnumerator0")
        (goto _label)))))

(event Input|ActionEvents|InputActionCrouch
  (params (Key :type Key%20Structure))
  (bind _returnvalue (Utilities|GetAnimInstance))
  ;[1 1 1] しゃがみ
  (:Pressed
    (Utilities|FlowControl|FlipFlop
      (:A
        (Utilities|CheckMovementCondition (Utilities|Struct|MakeS_MovementState (Variables|BOOL|GetRunning) false false false false false)
          (:DoLogic
            (bind _output_get (Variables|BOOL|SetCrouching true))
            ;;[0.04417 0 1] Interface呼び出し
            (Class|BPIAnimation|SetCrouch(Message) _returnvalue _output_get)
            (CallFunction|ChangeMovementType "NewEnumerator2"))))
      (:B
        (Utilities|CheckMovementCondition (Utilities|Struct|MakeS_MovementState (Variables|BOOL|GetRunning) false false false false false)
          (:DoLogic
            (bind _output_get_2 (Variables|BOOL|SetCrouching false))
            (Class|BPIAnimation|SetCrouch(Message) _returnvalue _output_get_2)
            (CallFunction|ChangeMovementType (Utilities|CorrectMovementType "NewEnumerator1" "NewEnumerator0" "NewEnumerator1"))))))
    (CallFunction|UpdateMovementState)))

(event Input|ActionEvents|InputActionJump
  (params (Key :type Key%20Structure))
  ;[1 1 1] ジャンプ処理(空中でジャンプできないようにbrach)
  (:Pressed
    (if (not (AI|Components|NavMovement|IsFalling (Variables|Character|GetCharacterMovement)))
      ;;[1 1 1] ジャンプ処理
      (Character|LaunchCharacter (|CalculateJumpForce) false false))))

(event Input|AxisEvents|InputAxisMoveForward/Backward
  (params (AxisValue :type Float%20%28single-precision%29))
  ;[1 0.2917 0.2917] 移動処理(GetControlRotationのYawだけを取っているのは下を向きながら移動したときに地面に進もうとするのを防ぐ為)
  (Pawn|Input|AddMovementInput (Math|Vector|GetForwardVector (Math|Rotator|MakeRotator 0.0 0.0 (.yaw (Pawn|GetControlRotation :!class /Script/Engine.Pawn)))) AxisValue false)
  (CallFunction|WalkCameraShake))

(event Input|AxisEvents|InputAxisMoveRight/Left
  (params (AxisValue :type Float%20%28single-precision%29))
  ;[1 0.2917 0.2917] 移動処理(GetControlRotationのYawだけを取っているのは下を向きながら移動したときに地面に進もうとするのを防ぐ為)
  (Pawn|Input|AddMovementInput (Math|Vector|GetRightVector (Math|Rotator|MakeRotator 0.0 0.0 (.yaw (Pawn|GetControlRotation :!class /Script/Engine.Pawn)))) AxisValue false)
  (CallFunction|WalkCameraShake))

(event Input|AxisEvents|InputAxisLookUp/Down
  (params (AxisValue :type Float%20%28single-precision%29))
  ;[1 0.2292 0.2292] 視点移動処理
  (Pawn|Input|AddControllerPitchInput AxisValue))

(event Input|AxisEvents|InputAxisLookRight/Left
  (params (AxisValue :type Float%20%28single-precision%29))
  ;[1 0.2292 0.2292] 視点移動処理
  (Pawn|Input|AddControllerYawInput AxisValue))

(event EventBeginPlay
  (Utilities|FlowControl|Sequence
    (:then_0
      ;[0.02547 0.02544 0.02604] 銃クラスをSpawnし、手に付ける。Spawn ACtor関数の、Classをいじる事でクラスを変えることが出来る
      (bind _returnvalue (Game|SpawnActorfromClass "/Game/BP/Actor/Weapon/AR4/BP_AR4.BP_AR4_C" (Math|Transform|MakeTransform "0, 0, 0" "0, 0, 0" "1,1,1") "AlwaysSpawn" 0 0)) ; 武器の生成
      (bind _output_get (Variables|REFERENCE|SetWeapon _returnvalue))
      (bind _weaponname (Default|Equip _output_get (Variables|Character|GetMesh) self))
      (Class|BPIAnimation|GetWeaponInfo(Message) (Utilities|GetAnimInstance) (Variables|REFERENCE|GetWeapon) _weaponname))))

(event EventTick
  (params (DeltaSeconds :type Float%20%28single-precision%29))
  (Utilities|FlowControl|Sequence
    (:then_0
      (bind (_direction _speed _pitch _yaw) (CallFunction|CalculateMovementValue))
      (Class|BPIAnimation|GetMovementValue(Message) (Utilities|GetAnimInstance) _direction _speed _pitch _yaw))))

(event Input|ActionEvents|InputActionAim
  (params (Key :type Key%20Structure :default "None"))
  ;[1 1 1] ADS(サイトを覗いて照準を合わせること)
  (:Pressed
    (Utilities|CheckMovementCondition (Utilities|Struct|MakeS_MovementState (Variables|BOOL|GetRunning) false false false (Variables|BOOL|GetReloading) (Variables|BOOL|GetHoldingGrenade)) ; Pressed(押されたとき)
      (:DoLogic
        (bind _output_get (Variables|BOOL|SetAiming true))
        ;;[0.1094 0.1094 0.1094] 銃クラス内のADS関数を呼び出し
        (Default|ADS (Variables|REFERENCE|GetWeapon) _output_get)
        (CallFunction|ChangeMovementType (Utilities|CorrectMovementType "NewEnumerator2" "NewEnumerator1" "NewEnumerator2")))))
  (:Released
    (Utilities|CheckMovementCondition (Utilities|Struct|MakeS_MovementState (Variables|BOOL|GetRunning) false false false (Variables|BOOL|GetReloading) (Variables|BOOL|GetHoldingGrenade)) ; Released(押してから離したとき)
      (:DoLogic
        (bind _output_get_2 (Variables|BOOL|SetAiming false))
        (Default|ADS (Variables|REFERENCE|GetWeapon) _output_get_2)
        (CallFunction|ChangeMovementType (Utilities|CorrectMovementType "NewEnumerator2" "NewEnumerator0" "NewEnumerator2"))))))

(event Input|ActionEvents|InputActionFire
  (params (Key :type Key%20Structure :default "None"))
  ;[1 1 1] Fire(発射・速度)
  (:Pressed
    (Utilities|CheckMovementCondition (Utilities|Struct|MakeS_MovementState (Variables|BOOL|GetRunning) false false false (Variables|BOOL|GetReloading) (Variables|BOOL|GetHoldingGrenade)) ; Released(押してから離したとき)
      (:DoLogic
        (Variables|BOOL|SetFireing false)
        (Utilities|Time|PauseTimerbyHandle (Variables|HANDLE|GetH_Fire))))))

(event Input|ActionEvents|InputActionReload
  (params (Key :type Key%20Structure :default "None"))
  (bind _returnvalue (Utilities|GetAnimInstance))
  ;[1 1 1] reload(弾薬を再装填)
  (:Pressed
    (Utilities|CheckMovementCondition (Utilities|Struct|MakeS_MovementState false false (Variables|BOOL|GetAiming) (Variables|BOOL|GetFireing) false (Variables|BOOL|GetHoldingGrenade)) ; Pressed(押されたとき)
      (:DoLogic
        (Variables|BOOL|SetReloading true)
        ;;[0.1134 0 1] 左手のIKを無効にするInterface
        (Class|BPIAnimation|SetLeftHandIKAlpha(Message) _returnvalue 0.0)
        ;;[0 0 0] リロードのAnimMontageをプレイ
        (bind _returnvalue_2 (Animation|Montage|MontagePlay _returnvalue "/Game/Imported/AnimStarterPack/Montage/RifleReloadMontage.RifleReloadMontage" 1.0 "MontageLength" 0.0 true))
        (Utilities|FlowControl|Delay _returnvalue_2)
        ;;[0.05332 0 1] Interface
        (Class|BPIAnimation|SetLeftHandIKAlpha(Message) (Utilities|GetAnimInstance) 1.0)))))

(event Input|ActionEvents|InputActionGrenade
  (params (Key :type Key%20Structure :default "None"))
  ;[1 1 1] Grenade
  (:Pressed
    (Utilities|CheckMovementCondition (Utilities|Struct|MakeS_MovementState false false (Variables|BOOL|GetAiming) (Variables|BOOL|GetFireing) (Variables|BOOL|GetReloading) false)) ; Pressed(押されたとき)\nDo Logic = グレネードを投げる
  )
  (:Released
    (Utilities|CheckMovementCondition (Utilities|Struct|MakeS_MovementState false false (Variables|BOOL|GetAiming) (Variables|BOOL|GetFireing) (Variables|BOOL|GetReloading) false)) ; Released(押してから離したとき)\nDo Logic = グレネードを投げる
  ))

(event Input|ActionEvents|InputActionFire
  (params (Key :type Key%20Structure :default "None"))
  (bind _weapon (Variables|REFERENCE|GetWeapon))
  ;[1 1 1] Fire(発射・速度)
  (:Pressed
    (Utilities|CheckMovementCondition (Utilities|Struct|MakeS_MovementState (Variables|BOOL|GetRunning) false false false (Variables|BOOL|GetReloading) (Variables|BOOL|GetHoldingGrenade)) ; Pressed(押されたとき)
      (:DoLogic
        (Variables|BOOL|SetFireing true)
        ;;[0.07812 0.07812 0.07812] 銃クラスのFire(発射)関数を一度呼び出し、Timer 処理。FireRate(発射速度)変数でループ
        (Default|Fire _weapon)
        (bind _returnvalue (Utilities|Time|SetTimerbyFunctionName _weapon "Fire" (Variables|/Game/BP/Actor/Weapon/BP_Weapon_Base.BP_Weapon_Base_C|GetFireRate _weapon) true))
        (Variables|HANDLE|SetH_Fire _returnvalue)))))